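; BP_Toilet_01 is an interactive toilet prop whose lid the player can raise and lower with the F key.
; A box trigger enables input while the player character overlaps it and disables it on exit.
; Each press flip-flops a timeline that plays or reverses, rolling the lid mesh up to 90 degrees.
; The construction script sets the lid's initial roll from a variable.
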(event `self.Box.OnComponentBeginOverlap`
  (params (OverlappedComponent :type "PrimitiveComponent Object Reference") (OtherActor :type "Actor Object Reference") (OtherComp :type "PrimitiveComponent Object Reference") (OtherBodyIndex :type Integer) (bFromSweep :type Boolean) (SweepResult :type "HitResult Structure (by ref)"))
  (if (== (`GameplayStatics.GetPlayerCharacter` 0) OtherActor)
    (`self.EnableInput` (`GameplayStatics.GetPlayerController` 0))))

(event `self.Box.OnComponentEndOverlap`
  (params (OverlappedComponent :type "PrimitiveComponent Object Reference") (OtherActor :type "Actor Object Reference") (OtherComp :type "PrimitiveComponent Object Reference") (OtherBodyIndex :type Integer))
  (if (== (`GameplayStatics.GetPlayerCharacter` 0) OtherActor)
    (`self.DisableInput` (`GameplayStatics.GetPlayerController` 0))))

(event `Key|F`
  (params (Key :type "Key Structure"))
  (:`Pressed`
    (`/Engine/EditorBlueprintResources/StandardMacros.FlipFlop`
      (:`A`
        (bind (_direction _newtrack_0) (`Timeline|Timeline_0` :!label _label)
          (:`Update`
            (`SceneComponent.K2_SetRelativeRotation` (`self.SM_Bathroom01_SM_ToiletLid_01`) (`KismetMathLibrary.MakeRotator` (* _newtrack_0 -90.0)) false false))))
      (:`B`
        (goto _label :!via `Reverse`)))))

(fn `UserConstructionScript`
  (`SceneComponent.K2_SetRelativeRotation` (`self.SM_Bathroom01_SM_ToiletLid_01`) (`KismetMathLibrary.MakeRotator` (`self.New Rotation X (Roll)`)) false false))