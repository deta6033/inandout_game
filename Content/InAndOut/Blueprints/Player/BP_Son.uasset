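; BP_Son is the Son player Blueprint, handling visual feedback for its pillow melee and report card ultimate.
; The melee event hides the foam dart gun, then a timeline sweeps the pillow pivot through a roll arc and hides the pillow afterward, without re-showing the gun.
; The ultimate event briefly shows a report card widget on screen.
; The construction script shrinks the actor to a child-sized scale.
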(event `self.BP_OnReportCardUltimate`
  (bind _returnvalue (`|CreateWidget` "/Game/InAndOut/UI/WBP_ReportCard.WBP_ReportCard_C"))
  (`UserWidget.AddToViewport` _returnvalue 0)
  (`KismetSystemLibrary.Delay` 1.2)
  (`Widget.RemoveFromParent` _returnvalue))

(event `self.ReceiveBeginPlay`)

(event `self.BP_OnPillowMelee`
  (`SceneComponent.SetVisibility` (`self.FoamDartGunMesh`) false false)
  (`SceneComponent.SetHiddenInGame` (`self.PillowSwingMesh`) false false)
  (bind (_direction _alpha) (`Timeline|TL_PillowSwing` :!via `PlayFromStart`)
    (:`Update`
      (`SceneComponent.K2_SetRelativeRotation` (`self.PillowPivot`) (`KismetMathLibrary.RLerp` (struct :`Yaw` 70.0) (struct :`Yaw` -70.0) _alpha) false false))
    (:`Finished`
      (`SceneComponent.SetHiddenInGame` (`self.PillowSwingMesh`) true false))))

(fn `UserConstructionScript`
  (`self.SetActorScale3D` (0.3 0.3 0.3)))